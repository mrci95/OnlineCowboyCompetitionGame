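; Lobby game mode that assigns player start points by overriding ChoosePlayerStart.
; With one player counted, it picks the untaken start whose object name is PlayerStartHost; with two, any untaken start.
; Each chosen start gets its PlayerStartTag set to Taken so it is not reused.
; Other player counts have no branch, and the event graph holds only disabled placeholder events.
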(event EventBeginPlay)

(event EventTick
  (params (DeltaSeconds :type Float%20%28single-precision%29)))

(fn ConstructionScript)

(fn ChoosePlayerStart
  (params (Player :type Controller%20Object%20Reference))
  (bind _returnvalue (Class|GameModeBase|GetNumPlayers))
  (switch int _returnvalue
    (:1
      (bind _outactors (Actor|GetAllActorsOfClass "/Script/Engine.PlayerStart"))
      (for _array_element _outactors
        (if (and (Utilities|Enum|Equal(Enum) (Utilities|GetObjectName _array_element) "PlayerStartHost") (Utilities|Name|NotEqual(Name) (Variables|/Script/Engine.PlayerStart|GetPlayerStartTag _array_element) "Taken"))
          (Variables|/Script/Engine.PlayerStart|SetPlayerStartTag _array_element "Taken")
          (return _array_element))))
    (:2
      (bind _outactors_2 (Actor|GetAllActorsOfClass "/Script/Engine.PlayerStart"))
      (for _array_element_2 _outactors_2
        (if (Utilities|Name|NotEqual(Name) (Variables|/Script/Engine.PlayerStart|GetPlayerStartTag _array_element_2) "Taken")
          (Variables|/Script/Engine.PlayerStart|SetPlayerStartTag _array_element_2 "Taken")
          (return _array_element_2))))))