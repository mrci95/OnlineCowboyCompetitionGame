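; BP_LobbyPawn is a lobby pawn that sets up its skeletal mesh according to the Player Start it occupies.
; On BeginPlay it finds the Player Start at its own location, within a small tolerance, and switches on that actor's object name.
; The client start mirrors the mesh on Y through negative scale, then both client and host starts toggle mesh visibility, propagating to children.
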(event EventBeginPlay
  (bind _outactors (Actor|GetAllActorsOfClass "/Script/Engine.PlayerStart"))
  (for _array_element _outactors
    (if (Math|Vector|Equal(Vector) (Transformation|GetWorldLocation (Variables|Transformation|GetRootComponent)) (Transformation|GetWorldLocation (Variables|/Script/Engine.Actor|GetRootComponent _array_element)) 1.0)
      (switch string (Utilities|GetObjectName _array_element)
        (:PlayerStartClient
          (Transformation|SetWorldScale3D (Variables|Default|GetSkeletalMesh) "1.000000,-1.000000,1.000000"))
        (:PlayerStartHost
          _))
      (Rendering|ToggleVisibility (Variables|Default|GetSkeletalMesh) true))))

(event Collision|EventActorBeginOverlap
  (params (OtherActor :type Actor%20Object%20Reference)))

(event EventTick
  (params (DeltaSeconds :type Float%20%28single-precision%29)))

(fn ConstructionScript)